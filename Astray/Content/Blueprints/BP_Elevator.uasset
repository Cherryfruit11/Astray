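; BP_Elevator is an elevator actor that responds to the first-person character entering and leaving trigger boxes.
; Overlapping Box plays the Elevator timeline after a short delay to move Cube along its ElevatorUp track, and leaving reverses it.
; A second trigger, LeftDoorBox, plays another timeline that sets the box's own relative location to a fixed origin, so door motion appears unfinished.
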(event `self.Box.OnComponentBeginOverlap`
  (params (OverlappedComponent :type "PrimitiveComponent Object Reference") (OtherActor :type "Actor Object Reference") (OtherComp :type "PrimitiveComponent Object Reference") (OtherBodyIndex :type Integer) (bFromSweep :type Boolean) (SweepResult :type "HitResult Structure (by ref)"))
  ;[1 1 1] Elevator Up and Down
  (cast `/Game/FirstPerson/Blueprints/BP_FirstPersonCharacter` OtherActor)
  (`KismetSystemLibrary.Delay` 0.2)
  (bind (_direction _elevator_up) (`Timeline|Elevator` :!label _label)
    (:`Update`
      (`SceneComponent.K2_SetRelativeLocation` (`self.Cube`) _elevator_up false false))))

(event `self.Box.OnComponentEndOverlap`
  (params (OverlappedComponent :type "PrimitiveComponent Object Reference") (OtherActor :type "Actor Object Reference") (OtherComp :type "PrimitiveComponent Object Reference") (OtherBodyIndex :type Integer))
  ;[1 1 1] Elevator Up and Down
  (cast `/Game/FirstPerson/Blueprints/BP_FirstPersonCharacter` OtherActor)
  (`KismetSystemLibrary.Delay` 0.2)
  (goto _label :!via `Reverse`))

(event `self.Left Door Box.OnComponentBeginOverlap`
  (params (OverlappedComponent :type "PrimitiveComponent Object Reference") (OtherActor :type "Actor Object Reference") (OtherComp :type "PrimitiveComponent Object Reference") (OtherBodyIndex :type Integer) (bFromSweep :type Boolean) (SweepResult :type "HitResult Structure (by ref)"))
  (cast `/Game/FirstPerson/Blueprints/BP_FirstPersonCharacter` OtherActor)
  (`KismetSystemLibrary.Delay` 0.2)
  (`Timeline|Timeline`
    (:`Update`
      (`SceneComponent.K2_SetRelativeLocation` (`self.Left Door Box`) (0.0 0.0 0.0) false false))))

(fn `UserConstructionScript`)