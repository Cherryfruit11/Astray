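; Elevator actor that carries the first-person character between two heights, starting down with its doors closed.
; When the character overlaps Box, it closes the doors, waits, then plays or reverses the Elevator timeline based on Isup to drive the actor's Z.
; When the timeline finishes, it opens the doors and flips Isup.
; Tick eases both doors toward hard-coded transforms with a DeltaSeconds-alpha lerp, steered by DoorsOpen and DoorsMoving, snapping them once close.
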(event `self.Box.OnComponentBeginOverlap`
  (params (OverlappedComponent :type "PrimitiveComponent Object Reference") (OtherActor :type "Actor Object Reference") (OtherComp :type "PrimitiveComponent Object Reference") (OtherBodyIndex :type Integer) (bFromSweep :type Boolean) (SweepResult :type "HitResult Structure (by ref)"))
  ;[1 1 1] Elevator Up and Down
  (cast `/Game/FirstPerson/Blueprints/BP_FirstPersonCharacter` OtherActor)
  (`self.CloseDoors`)
  (`KismetSystemLibrary.Delay` 5.0)
  (if (`self.isup`)
    (bind (_direction _newtrack_1) (`Timeline|Elevator` :!via `ReverseFromEnd` :!label _label)
      (:`Update`
        (`self.K2_SetActorLocation` (`KismetMathLibrary.MakeVector` (.x (`self.K2_GetActorLocation`)) (.y (`self.K2_GetActorLocation`)) _newtrack_1)))
      (:`Finished`
        (`self.OpenDoors`)
        (set `self.isup` (not (`self.isup`)))))
    (else
      (goto _label :!via `PlayFromStart`))))

(event `self.ReceiveBeginPlay`
  ;[1 1 1] Begin Event (Set Doors open and close to false)
  (set `self.isup` false)
  (set `self.Doors Open` false)
  (set `self.Doors Moving` false))

(event `self.ReceiveTick`
  (params (DeltaSeconds :type "Float (single-precision)"))
  (bind _returnvalue (`KismetMathLibrary.MakeTransform` (-90.0 120.0 125.0) (struct :`Roll` 90.0) (1.8 3.5 0.135)))
  (bind _returnvalue_2 (`KismetMathLibrary.MakeTransform` (-250.0 120.0 125.0) (struct :`Roll` 90.0) (1.8 3.5 0.135)))
  (bind _returnvalue_3 (`KismetMathLibrary.MakeTransform` (250.0 120.0 125.0) (struct :`Roll` 90.0) (1.8 3.5 0.135)))
  (bind _returnvalue_4 (`KismetMathLibrary.MakeTransform` (90.0 120.0 125.0) (struct :`Roll` 90.0) (1.8 3.5 0.135)))
  (bind _returnvalue_5 (`KismetMathLibrary.TLerp` (`SceneComponent.GetRelativeTransform` (`self.Left Door`)) _returnvalue DeltaSeconds))
  (bind _returnvalue_6 (`KismetMathLibrary.TLerp` (`SceneComponent.GetRelativeTransform` (`self.Right Door`)) _returnvalue_3 DeltaSeconds))
  (if (`self.Doors Moving`)
    (if (`self.Doors Open`)
      ;[1 1 1] Open-Moving
      (`SceneComponent.K2_SetRelativeTransform` (`self.Right Door`) _returnvalue_6 false false)
      (`SceneComponent.K2_SetRelativeTransform` (`self.Left Door`) (`KismetMathLibrary.TLerp` (`SceneComponent.GetRelativeTransform` (`self.Left Door`)) _returnvalue_2 DeltaSeconds) false false)
      (if (< (`KismetMathLibrary.Vector_Distance` (.location _returnvalue_6) (.location _returnvalue_3)) 0.1)
        (set `self.Doors Moving` false))
      (else
        ;[1 1 1] Closed-Moving
        (`SceneComponent.K2_SetRelativeTransform` (`self.Right Door`) (`KismetMathLibrary.TLerp` (`SceneComponent.GetRelativeTransform` (`self.Right Door`)) _returnvalue_4 DeltaSeconds) false false)
        (`SceneComponent.K2_SetRelativeTransform` (`self.Left Door`) _returnvalue_5 false false)
        (if (< (`KismetMathLibrary.Vector_Distance` (.location _returnvalue_5) (.location _returnvalue)) 0.1)
          (set `self.Doors Moving` false))))
    (elif (`self.Doors Open`)
      ;[1 1 1] Open
      (`SceneComponent.K2_SetRelativeTransform` (`self.Right Door`) _returnvalue_3 false false)
      (`SceneComponent.K2_SetRelativeTransform` (`self.Left Door`) _returnvalue_2 false false)
      (else
        ;[1 1 1] Closed
        (`SceneComponent.K2_SetRelativeTransform` (`self.Right Door`) _returnvalue_4 false false)
        (`SceneComponent.K2_SetRelativeTransform` (`self.Left Door`) _returnvalue false false)))))

(event `OpenDoors`
  (set `self.Doors Moving` true)
  (set `self.Doors Open` true))

(event `CloseDoors`
  (set `self.Doors Moving` true)
  (set `self.Doors Open` false))

(fn `UserConstructionScript`)